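; Lightning actor that drives a Niagara beam toward randomly chosen ForceSphere_BP actors in the level.
; Every tick it gathers all ForceSphere_BP actors and, after an index validity check, picks one at random.
; It writes that sphere's root location, relative to the Niagara component, into User.Beam End, so the beam can jump between spheres each frame.
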(event `self.ReceiveBeginPlay`)

(event `self.ReceiveTick`
  (params (DeltaSeconds :type "Float (single-precision)"))
  (bind _outactors (`GameplayStatics.GetAllActorsOfClass` "/Game/ForceSphere_BP.ForceSphere_BP_C"))
  (bind _returnvalue (`KismetMathLibrary.RandomIntegerInRange` 0 (- (`KismetArrayLibrary.Array_Length` _outactors) 1)))
  (if (`KismetArrayLibrary.Array_IsValidIndex` _outactors _returnvalue)
    (`NiagaraComponent.SetVariableVec3` (`self.Niagara`) "User.Beam End" (- (`SceneComponent.K2_GetComponentLocation` (`Actor.RootComponent` (`|GetArrayItem` _outactors _returnvalue))) (`SceneComponent.K2_GetComponentLocation` (`self.Niagara`))))))

(fn `UserConstructionScript`)