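; Ground spike trap actor that damages pawns stepping into its trigger box.
; On overlap begin, the skeletal mesh plays a one-shot spike-up animation, then damage is applied to that pawn after a short delay.
; When a pawn leaves the box, the mesh plays the spike-down animation.
; Damage lands even if the pawn exits during the delay, since overlap is not rechecked.
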(event `self.TriggerBox.OnComponentBeginOverlap`
  (params (OverlappedComponent :type "PrimitiveComponent Object Reference") (OtherActor :type "Actor Object Reference") (OtherComp :type "PrimitiveComponent Object Reference") (OtherBodyIndex :type Integer) (bFromSweep :type Boolean) (SweepResult :type "HitResult Structure (by ref)"))
  (bind _aspawn (cast `Pawn` OtherActor))
  (`SkeletalMeshComponent.PlayAnimation` (`self.SkeletalMesh`) "/Game/Props/Traps/GroundTrap/GroundSpikes_Anim_Armature_SpikeUp.GroundSpikes_Anim_Armature_SpikeUp" false)
  (`KismetSystemLibrary.Delay` 0.2)
  (`GameplayStatics.ApplyDamage` _aspawn (`self.damage`) null self))

(event `self.TriggerBox.OnComponentEndOverlap`
  (params (OverlappedComponent :type "PrimitiveComponent Object Reference") (OtherActor :type "Actor Object Reference") (OtherComp :type "PrimitiveComponent Object Reference") (OtherBodyIndex :type Integer))
  (cast `Pawn` OtherActor)
  (`SkeletalMeshComponent.PlayAnimation` (`self.SkeletalMesh`) "/Game/Props/Traps/GroundTrap/GroundSpikes_Anim_Armature_SpikeDown.GroundSpikes_Anim_Armature_SpikeDown" false))

(fn `UserConstructionScript`)