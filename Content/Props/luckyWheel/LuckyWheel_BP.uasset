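; Lucky wheel prop that spins on its own in an endless loop, with no player interaction wired up.
; BeginPlay gives RotatingMovement a random yaw rate, which Tick lowers by a fixed step each frame, so slowdown depends on frame rate.
; Once the rate runs out, it waits a second and spins again.
; Interact is empty, and an alternative timeline-driven mesh rotation loop is left disconnected.
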(event `self.ReceiveBeginPlay`
  (set `RotatingMovementComponent.RotationRate` (`KismetMathLibrary.MakeRotator` 0.0 0.0 (`KismetMathLibrary.RandomFloatInRange` 60.0 360.0)) (`self.RotatingMovement`) :!label _label)
  (set `self.bIsWheelRotating` true))

(event `self.ReceiveTick`
  (params (DeltaSeconds :type "Float (single-precision)"))
  (bind _rotatingmovement (`self.RotatingMovement`))
  (bind _returnvalue (- (.yaw (`RotatingMovementComponent.RotationRate` _rotatingmovement)) 1.0))
  (if (`self.bIsWheelRotating`)
    (set `RotatingMovementComponent.RotationRate` (`KismetMathLibrary.MakeRotator` 0.0 0.0 _returnvalue) _rotatingmovement)
    (if (< _returnvalue 0.0)
      (set `self.bIsWheelRotating` false)
      (`KismetSystemLibrary.Delay` 1.0)
      (goto _label))))

(event `/Game/Interaction_BPI.Interact`)

(fn `UserConstructionScript`)