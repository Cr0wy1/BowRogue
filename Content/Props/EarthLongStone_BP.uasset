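; Earth long stone prop that rises after spawning and launches characters who touch it while it is still rising.
; Shortly after BeginPlay, the StoneZLoc timeline drives the static mesh's relative location and sets IsStoneUp when finished.
; Until that flag is set, Box overlaps launch an AdvancedCharacter upward and along the stone's forward vector, printing a debug string.
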(event `self.ReceiveBeginPlay`
  (`KismetSystemLibrary.Delay` 0.5)
  (bind (_direction _newtrack_1) (`Timeline|StoneZLoc`)
    (:`Update`
      (`SceneComponent.K2_SetRelativeLocation` (`self.StaticMesh`) _newtrack_1 false false))
    (:`Finished`
      (set `self.isStoneUp` true))))

(event `self.Box.OnComponentBeginOverlap`
  (params (OverlappedComponent :type "PrimitiveComponent Object Reference") (OtherActor :type "Actor Object Reference") (OtherComp :type "PrimitiveComponent Object Reference") (OtherBodyIndex :type Integer) (bFromSweep :type Boolean) (SweepResult :type "HitResult Structure (by ref)"))
  (bind _asadvanced_character (cast `AdvancedCharacter` OtherActor))
  (if (not (`self.isStoneUp`))
    (`Character.LaunchCharacter` _asadvanced_character (`KismetMathLibrary.MakeVector` (.x (* (`KismetMathLibrary.GetForwardVector` (`self.K2_GetActorRotation`)) 300.0)) (.y (* (`KismetMathLibrary.GetForwardVector` (`self.K2_GetActorRotation`)) 300.0)) 1000.0) false false)
    (`KismetSystemLibrary.PrintString` "Hello")))

(fn `UserConstructionScript`)