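; Orbit pivot for the Earth Elemental boss's attacks that carries an attached actor in a circle around itself.
; AttachActor sets orbit speed and spring arm length, then snaps the given actor onto the arm; BeginPlay also attaches any OrbitActor already set.
; A timeline started at BeginPlay animates the arm's height, while Tick adds OrbitSpeed as yaw every frame without delta-time scaling.
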(event `self.ReceiveBeginPlay`
  (bind _orbitactor (`self.OrbitActor`))
  (if (`KismetSystemLibrary.IsValid` _orbitactor)
    (`self.K2_AttachToComponent` _orbitactor (`self.SpringArm`) "None" "SnapToTarget" "KeepRelative" "KeepRelative" true)
    (bind (_direction _zloc) (`Timeline|ArmZLoc` :!label _label)
      (:`Update`
        (`SceneComponent.K2_SetRelativeLocation` (`self.SpringArm`) (`KismetMathLibrary.MakeVector` 0.0 0.0 _zloc) false false)))
    (else
      (goto _label))))

(event `self.ReceiveTick`
  (params (DeltaSeconds :type "Float (single-precision)"))
  (`SceneComponent.K2_AddRelativeRotation` (`self.SpringArm`) (`KismetMathLibrary.MakeRotator` 0.0 0.0 (`self.OrbitSpeed`)) false false))

(fn `AttachActor`
  (params (Actor :type "Actor Object Reference") (ArmLength :type "Float (double-precision)" :default 1000.0) (OrbitSpeed :type "Float (double-precision)"))
  (bind _springarm (`self.SpringArm`))
  (set `self.OrbitSpeed` OrbitSpeed)
  (set `SpringArmComponent.TargetArmLength` ArmLength _springarm)
  (if (`KismetSystemLibrary.IsValid` Actor)
    (bind _output_get (set `self.OrbitActor` Actor))
    (`self.K2_AttachToComponent` _output_get _springarm "None" "SnapToTarget" "KeepRelative" "KeepRelative" true)))

(fn `UserConstructionScript`)