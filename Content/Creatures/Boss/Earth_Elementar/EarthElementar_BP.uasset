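; Earth elemental boss character that plays a build-up montage on spawn, then has its AI controller run the EarthElementar behavior tree once the montage completes.
; It keeps a queue of stone projectiles, filled through AddStoneProjectile.
; PullProjectile removes the oldest stone, detaches it and returns it to the caller.
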(event `self.ReceiveBeginPlay`
  (`|PlayMontage` (`self.Mesh`) "/Game/Creatures/Boss/Earth_Elementar/earth_elementar_Anim_Armature_buildUp_MTG.earth_elementar_Anim_Armature_buildUp_MTG"
    (:`OnCompleted`
      (bind _asaicontroller (cast `AIController` (`self.GetController`)))
      (`AIController.RunBehaviorTree` _asaicontroller "/Game/Creatures/Boss/Earth_Elementar/AI/EarthElementar_BT.EarthElementar_BT"))))

(fn `AddStoneProjectile`
  (params (NewProjectile :type "Projectile Object Reference"))
  (`KismetArrayLibrary.Array_Add` (`self.StoneProjectiles`) NewProjectile))

(fn `PullProjectile`
  (returns (Projectile :type "Projectile Object Reference"))
  (bind _stoneprojectiles (`self.StoneProjectiles`))
  (if (> (`KismetArrayLibrary.Array_Length` _stoneprojectiles) 0)
    (bind _output_get (set `self.PulledProjectile` (`|GetArrayItem` _stoneprojectiles)))
    (`KismetArrayLibrary.Array_Remove` _stoneprojectiles)
    (`self.K2_DetachFromActor` _output_get "KeepRelative" "KeepRelative" "KeepRelative")
    (return _output_get)))

(fn `UserConstructionScript`)