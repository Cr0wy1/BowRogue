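; GeoCube_BP is a cube geometry creature with a point light and a physics-driven mesh.
; On BeginPlay it copies the light's color into the mesh materials' emission parameter so both match.
; Each Tick, while vertical velocity is below a small threshold, it applies a mass-independent upward acceleration that counters gravity.
; Leftover logic for targeting the player and making delayed, spinning jumps is disconnected and never runs.
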(event `self.ReceiveBeginPlay`
  (`MeshComponent.SetVectorParameterValueOnMaterials` (`self.meshComp`) "EmissionColor" (`KismetMathLibrary.Conv_LinearColorToVector` (`LightComponentBase.GetLightColor` (`self.PointLight`)))))

(event `self.ReceiveTick`
  (params (DeltaSeconds :type "Float (single-precision)"))
  (if (< (.z (`self.GetVelocity`)) 10.0)
    (`PrimitiveComponent.AddForce` (`self.meshComp`) (0.0 0.0 800.0) "None" true)))

(fn `UserConstructionScript`)