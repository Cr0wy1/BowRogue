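; Cube creature pawn that chases the player by pushing its Cube component with physics forces.
; From BeginPlay, the AddmoveForce timeline applies force toward player pawn 0 on each update, then restarts after a short delay.
; Cube hits and timeline completions only print debug text; damage handling is empty.
; Unwired leftovers hold alternative approaches: behavior tree, timeline-driven mesh rotation, impulse movement and physics-to-actor transform syncing.
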(event `self.ReceiveBeginPlay`
  (bind _cube (`self.Cube`))
  (`Timeline|AddmoveForce` :!via `PlayFromStart` :!label _label
    (:`Update`
      (`PrimitiveComponent.AddForce` _cube (* (`KismetMathLibrary.Normal` (- (`self.K2_GetActorLocation` (`GameplayStatics.GetPlayerPawn` 0)) (`SceneComponent.K2_GetComponentLocation` _cube))) 300000.0) "None" false))
    (:`Finished`
      (`KismetSystemLibrary.PrintString` "added force")
      (`KismetSystemLibrary.Delay` 0.1)
      (goto _label :!via `PlayFromStart`))))

(event `self.OnTakeDamage`
  (params (damageAmount :type "Float (single-precision)")))

(event `self.Cube.OnComponentHit`
  (params (HitComponent :type "PrimitiveComponent Object Reference") (OtherActor :type "Actor Object Reference") (OtherComp :type "PrimitiveComponent Object Reference") (NormalImpulse :type "Vector Structure") (Hit :type "HitResult Structure (by ref)"))
  (`KismetSystemLibrary.PrintString` (`KismetSystemLibrary.GetDisplayName` OtherActor)))

(fn `UserConstructionScript`)