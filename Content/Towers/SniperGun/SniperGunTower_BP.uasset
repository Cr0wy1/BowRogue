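; Sniper gun tower that fires sniper projectiles and tilts its gun mesh.
; OnFire spawns a scaled-down SniperProjectile_BP at the Arrow component's world location and rotation.
; Each Tick, GetUpdateRotationAmount, defined outside this graph, evaluates StaticMesh1's relative transform and, when it returns true, only the pitch of its result is added to that mesh, leaving yaw and roll untouched.
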(event `self.OnFire`
  (bind (_returnvalue_location _returnvalue_rotation) (`KismetMathLibrary.BreakTransform` (`SceneComponent.K2_GetComponentToWorld` (`self.Arrow`))))
  (`|SpawnActorFromClass` "/Game/Towers/SniperGun/SniperProjectile_BP.SniperProjectile_BP_C" (`KismetMathLibrary.MakeTransform` _returnvalue_location _returnvalue_rotation (0.2 0.2 0.2)) "Undefined" "OverrideRootScale" null null))

(event `self.ReceiveTick`
  (params (DeltaSeconds :type "Float (single-precision)"))
  (bind _staticmesh1 (`self.StaticMesh1`))
  (bind (_updaterotation _returnvalue) (`self.GetUpdateRotationAmount` DeltaSeconds (`SceneComponent.RelativeRotation` _staticmesh1) (`SceneComponent.RelativeLocation` _staticmesh1)))
  (if _returnvalue
    (`SceneComponent.K2_AddRelativeRotation` (`self.StaticMesh1`) (`KismetMathLibrary.MakeRotator` 0.0 (.pitch _updaterotation)) false false)))

(fn `UserConstructionScript`)